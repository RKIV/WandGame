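; Gameplay player controller that handles LAN lobby creation, session joining and spell spawning for a wizard-style game.
; Input actions launch a lobby through GameInfoInstance or search sessions and join the first found.
; AddToCastVector records body parts (shoulders, hips) as numeric codes in CastVector, using -1 as empty.
; ServerSpawnSpell uses the vector's X to spawn Stupify or Expelliarmus and resets it on authority; Fireball spawning is disconnected.
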(event `InputAction|CreateSession`
  (params (Key :type "Key Structure"))
  ;[1 1 1] Create Session
  (:`Pressed`
    (`KismetSystemLibrary.PrintString` "Attempting to create session")
    (`self.SetReplicates` false)
    (bind _asgame_info_instance (cast `/Game/Blueprints/AllLevels/GameInfoInstance` (`GameplayStatics.GetGameInstance`)))
    (`/Game/Blueprints/AllLevels/GameInfoInstance.LaunchLobby` _asgame_info_instance 5 true "Test")))

(event `InputAction|JoinSession`
  (params (Key :type "Key Structure"))
  ;[1 1 1] Find Session
  (:`Pressed`
    (`KismetArrayLibrary.Array_Clear` (`self.FoundSessions`))
    (bind _results (`FindSessionsCallbackProxyAdvanced.FindSessionsAdvanced` self 20 false "AllServers")
      (:`OnSuccess`
        (bind _output_get (set `self.FoundSessions` _results))
        (if (> (`KismetArrayLibrary.Array_Length` _output_get) 0)
          (bind _asgame_info_instance (cast `/Game/Blueprints/AllLevels/GameInfoInstance` (`GameplayStatics.GetGameInstance`)))
          (`/Game/Blueprints/AllLevels/GameInfoInstance.JoinServer` _asgame_info_instance (`|GetArrayItem` _output_get)) ; Join First Session Found
          (else
            (`KismetSystemLibrary.PrintString` "No sessions found"))))
      (:`OnFailure`
        (`KismetSystemLibrary.PrintString` "Failure to find sessions")))))

(event `ServerSpawnSpell`
  (params (SpawnTransform :type "Transform Structure"))
  (bind _castvector_x (`KismetMathLibrary.BreakVector` (`self.CastVector`)))
  (bind _returnvalue (`KismetMathLibrary.FTrunc` _castvector_x))
  ;[1 1 1] Multicast Spawn Spell
  (`KismetSystemLibrary.PrintString` (`KismetStringLibrary.Conv_IntToString` _returnvalue))
  (switch `int` _returnvalue
    (:`Default`
      (`KismetSystemLibrary.PrintString` "Not Actually spawning spell" :!label _label))
    (:`0`
      (`|SpawnActorFromClass` "/Game/Blueprints/Spells/Stupify.Stupify_C" SpawnTransform "AdjustIfPossibleButDontSpawnIfColliding" "OverrideRootScale" null null))
    (:`1`
      (`|SpawnActorFromClass` "/Game/Blueprints/Spells/Expelliarmus.Expelliarmus_C" SpawnTransform "AdjustIfPossibleButDontSpawnIfColliding" "OverrideRootScale" null null))
    (:`2`
      (goto _label)))
  (`/Engine/EditorBlueprintResources/ActorMacros.Switch Has Authority`
    (:`Authority`
      (`KismetSystemLibrary.PrintString` "Am Authority")
      (set `self.CastVector` (-1.0 -1.0 -1.0)))
    (:`Remote`
      _))
  (`KismetSystemLibrary.PrintString` "Spawning Projectile"))

(fn `AddToCastVector`
  (params (BodyPart :type String))
  (bind (_castvector_x _castvector_y _castvector_z) (`KismetMathLibrary.BreakVector` (`self.CastVector`)))
  (bind (_castvector_x_2 _castvector_y_2 _castvector_z_2) (`KismetMathLibrary.BreakVector` (`self.CastVector`)))
  (bind _castvector_x_3 (`KismetMathLibrary.BreakVector` (`self.CastVector`)))
  (switch `string` BodyPart
    (:`left_shoulder`
      (if (== _castvector_x_3 -1.0)
        (set `self.CastVector` (`KismetMathLibrary.MakeVector` 0.0 _castvector_y_2 _castvector_z_2))
        (else
          (set `self.CastVector` (`KismetMathLibrary.MakeVector` _castvector_x_2 0.0 _castvector_y_2)))))
    (:`right_shoulder`
      (if (== _castvector_x_3 -1.0)
        (set `self.CastVector` (`KismetMathLibrary.MakeVector` 1.0 _castvector_y_2 _castvector_z_2))
        (else
          (set `self.CastVector` (`KismetMathLibrary.MakeVector` _castvector_x_2 1.0 _castvector_z_2)))))
    (:`left_hip`
      (if (== _castvector_x_3 -1.0)
        (set `self.CastVector` (`KismetMathLibrary.MakeVector` 2.0 _castvector_y _castvector_z))
        (else
          (set `self.CastVector` (`KismetMathLibrary.MakeVector` _castvector_x 2.0 _castvector_z)))))
    (:`right_hip`
      (if (== _castvector_x_3 -1.0)
        (set `self.CastVector` (`KismetMathLibrary.MakeVector` 3.0 _castvector_y _castvector_z))
        (else
          (set `self.CastVector` (`KismetMathLibrary.MakeVector` _castvector_x 3.0 _castvector_z)))))))

(fn `UserConstructionScript`)